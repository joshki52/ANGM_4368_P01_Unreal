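; Player construction tool, a child actor of the first-person character, that places, rotates and removes rooms in build mode.
; A hologram preview snaps to a grid ahead of the camera, cycles through the game mode's unlocked rooms and turns red when overlapping a room detector.
; Overlap blocks construction and marks the room for deletion, refused while the player is inside.
; Preview meshes come from briefly spawning each room class off-map on every update.
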(event `Enter Build Preview`
  (bind _preview (`self.Preview`))
  ; Build Preview
  (`self.Print Debug` "Enter Build Preview")
  (`SceneComponent.SetVisibility` _preview true false)
  (`PrimitiveComponent.SetCollisionEnabled` _preview "QueryOnly")
  (`self.Update Room Type`)
  (`self.Update Build Preview`))

(event `Player Updated`
  ; Player Inputs
  ;; Any Player Movement (aiming with mouse, moving with keyboard)
  (if (`self.Build Mode`)
    (`self.Update Build Preview`)))

(event `Update Build Preview`
  ; Build Preview
  (`self.Get Preview Mesh (Janky)`)
  (bind _location (`self.Calculate Preview Location` (`self.Player Camera`) (`self.Player Root Component`) (`self.Construction Unit Scale`) (`self.Target Distance`)))
  (`SceneComponent.K2_SetWorldLocation` (`self.Preview`) _location false true)
  (if (`self.Is Preview Overlapping`)
    (`PrimitiveComponent.SetMaterial` (`self.Preview`) 0 "/Game/_Game/Materials/MI_Hologram_Red.MI_Hologram_Red")
    (else
      (`PrimitiveComponent.SetMaterial` (`self.Preview`) 0 "/Game/_Game/Materials/MI_Hologram_Blue.MI_Hologram_Blue"))))

(event `Toggle Build Mode`
  ; Player Inputs
  ;; Toggle Build Mode
  (if (`self.Build Mode`)
    (set `self.Build Mode` false)
    (`self.Exit Build Preview`)
    (else
      (set `self.Build Mode` true)
      (`self.Enter Build Preview`))))

(event `Exit Build Preview`
  (bind _preview (`self.Preview`))
  ; Build Preview
  (`self.Print Debug` "Exit Build Preview")
  (`SceneComponent.SetVisibility` _preview false false)
  (`PrimitiveComponent.SetCollisionEnabled` _preview "NoCollision"))

(event `Next Room Type`
  ; Player Inputs
  ;; Select Next Room Type
  (if (`self.Build Mode`)
    (bind _result (`/Engine/EditorBlueprintResources/StandardMacros.IncrementInt` (`self.Construct Room Index`))
      (:`  `
        (if (> _result (- (`KismetArrayLibrary.Array_Length` (`/Game/_Game/Player/BP_FirstPersonGameMode.Unlocked Rooms` (`self.First Person Game Mode`))) 1))
          (set `self.Construct Room Index` 0))
        (`self.Update Room Type`)
        (`self.Update Build Preview`)))))

(event `self.Preview.OnComponentBeginOverlap`
  (params (OverlappedComponent :type "PrimitiveComponent Object Reference") (OtherActor :type "Actor Object Reference") (OtherComp :type "PrimitiveComponent Object Reference") (OtherBodyIndex :type Integer) (bFromSweep :type Boolean) (SweepResult :type "HitResult Structure (by ref)"))
  ; Test if Preview is Clipping
  (bind _result (`self.Test if Overlapped Actor is Room` OtherActor OtherComp))
  (if _result
    (set `self.Is Preview Overlapping` true)
    (bind _asbp_room_parent (cast `/Game/_Game/Blueprints/Rooms/BP_Room_Parent` OtherActor))
    (set `self.Last Overlapped Room` _asbp_room_parent)))

(event `Previous Room Type`
  ; Player Inputs
  ;; Select Previous Room Type
  (if (`self.Build Mode`)
    (bind _result (`/Engine/EditorBlueprintResources/StandardMacros.DecrementInt` (`self.Construct Room Index`))
      (:`  `
        (if (< _result 0)
          (set `self.Construct Room Index` (- (`KismetArrayLibrary.Array_Length` (`/Game/_Game/Player/BP_FirstPersonGameMode.Unlocked Rooms` (`self.First Person Game Mode`))) 1)))
        (`self.Update Room Type`)
        (`self.Update Build Preview`)))))

(event `self.Preview.OnComponentEndOverlap`
  (params (OverlappedComponent :type "PrimitiveComponent Object Reference") (OtherActor :type "Actor Object Reference") (OtherComp :type "PrimitiveComponent Object Reference") (OtherBodyIndex :type Integer))
  ; Test if Preview is Clipping
  (bind _result (`self.Test if Overlapped Actor is Room` OtherActor OtherComp))
  (if _result
    (set `self.Is Preview Overlapping` false)))

(event `Rotate Right`
  ; Player Inputs
  ;; Rotate Preview +90°
  (`SceneComponent.K2_AddWorldRotation` (`self.Preview`) (struct :`Yaw` 90.0) false false)
  (`self.Update Room Type` :!label _label)
  (`self.Update Build Preview`))

(event `Rotate Left`
  ; Player Inputs
  ;; Rotate Preview -90°
  (`SceneComponent.K2_AddWorldRotation` (`self.Preview`) (struct :`Yaw` -90.0) false false)
  (goto _label))

(event `Construct Room`
  ; Player Inputs
  ;; Construct Room
  (if (`self.Build Mode`)
    (if (`self.Is Preview Overlapping`)
      (`self.Print Debug` "Cannot construct; a room is already occupying this location.")
      (else
        (`|SpawnActorFromClass` (`self.Room Type`) (`SceneComponent.K2_GetComponentToWorld` (`self.Preview`)) "Undefined" "MultiplyWithRoot" null null)))
    (`self.Update Build Preview`)))

(event `Deconstruct Room`
  ; Player Inputs
  ;; Deconstruct Room
  (if (`self.Build Mode`)
    (if (`self.Is Preview Overlapping`)
      (bind _asbp_first_person_character (cast `/Game/_Game/Player/BP_FirstPersonCharacter` (`GameplayStatics.GetPlayerCharacter` 0))
        (:`then`
          (if (== (`KismetArrayLibrary.Array_Find` (`/Game/_Game/Player/BP_FirstPersonCharacter.Overlapping Rooms` _asbp_first_person_character) (`self.Last Overlapped Room`)) -1)
            (`self.K2_DestroyActor` (`self.Last Overlapped Room`))
            (else
              (`self.Print Debug` "Cannot deconstruct; player is currently inside room")))
          (`self.Update Build Preview`))
        (:`CastFailed`
          (`self.Print Debug` "Player character incorrectly referenced!"))))))

(fn `Calculate Preview Location`
  (params (`Player Camera` :type "CameraComponent Object Reference") (`Root Scene Component` :type "SceneComponent Object Reference") (`Unit Scale` :type Integer) (`Target Distance` :type Integer))
  (returns (Location :type "Vector Structure"))
  (bind (_returnvalue_x _returnvalue_y _returnvalue_z) (`KismetMathLibrary.BreakVector` (/ (+ (* `Target Distance` (`SceneComponent.GetForwardVector` `Player Camera`)) (`SceneComponent.K2_GetComponentLocation` `Root Scene Component`)) `Unit Scale`)))
  (return (* `Unit Scale` (`KismetMathLibrary.MakeVector` (`KismetMathLibrary.Conv_IntToDouble` (`KismetMathLibrary.Round` _returnvalue_x)) (`KismetMathLibrary.Conv_IntToDouble` (`KismetMathLibrary.Round` _returnvalue_y)) (`KismetMathLibrary.Conv_IntToDouble` (`KismetMathLibrary.Round` _returnvalue_z))))))

(fn `Get Game Mode`
  (bind _asbp_first_person_game_mode (cast `/Game/_Game/Player/BP_FirstPersonGameMode` (`GameplayStatics.GetGameMode`))
    (:`then`
      (set `self.First Person Game Mode` _asbp_first_person_game_mode))
    (:`CastFailed`
      (`KismetSystemLibrary.PrintString` "Incorrectly referenced game mode!"))))

(fn `Get Player Component References`
  (bind _asbp_first_person_character (cast `/Game/_Game/Player/BP_FirstPersonCharacter` (`self.GetParentActor`))
    (:`then`
      (set `self.Player Root Component` (`Actor.RootComponent` _asbp_first_person_character))
      (set `self.Player Camera` (`/Game/_Game/Player/BP_FirstPersonCharacter.FirstPersonCamera` _asbp_first_person_character)))
    (:`CastFailed`
      (`self.Print Debug` "Could not reference player component!"))))

(fn `Get Preview Mesh (Janky)`
  (bind _returnvalue (`|SpawnActorFromClass` (`self.Room Type`) (`KismetMathLibrary.MakeTransform` (0.0 0.0 -100000.0)) "Undefined" "MultiplyWithRoot" null null)) ; Cannot reference specific component from class alone,\nactor must exist in world in order to read data
  (bind _output_get (set `self.Preview Mesh` (`StaticMeshComponent.StaticMesh` (`/Game/_Game/Blueprints/Rooms/BP_Room_Parent.Room Mesh` _returnvalue))))
  (`self.K2_DestroyActor` _returnvalue)
  (`StaticMeshComponent.SetStaticMesh` (`self.Preview`) _output_get))

(fn `Print Debug`
  (params (String :type String))
  (if (`self.Print Debug String`)
    (`KismetSystemLibrary.PrintString` String)))

(fn `Test if Overlapped Actor is Room`
  (params (`Other Actor` :type "Actor Object Reference") (`Other Component` :type "PrimitiveComponent Object Reference"))
  (returns (Result :type Boolean))
  (if (`KismetMathLibrary.ClassIsChildOf` (`GameplayStatics.GetObjectClass` `Other Actor`) "/Game/_Game/Blueprints/Rooms/BP_Room_Parent.BP_Room_Parent_C")
    (bind _asbp_room_parent (cast `/Game/_Game/Blueprints/Rooms/BP_Room_Parent` `Other Actor`))
    (return (== (`/Game/_Game/Blueprints/Rooms/BP_Room_Parent.Room Detector` _asbp_room_parent) `Other Component`))))

(fn `Update Room Type`
  (bind _output_get (set `self.Room Type` (`|GetArrayItem` (`/Game/_Game/Player/BP_FirstPersonGameMode.Unlocked Rooms` (`self.First Person Game Mode`)) (`self.Construct Room Index`))))
  (`self.Print Debug` (`KismetSystemLibrary.GetClassDisplayName` _output_get)))

(fn `UserConstructionScript`
  (`self.Get Game Mode`)
  (`self.Get Player Component References`))