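; BP_Wall_Generic is a wall actor that removes itself from view and collision while it overlaps another wall of the same class.
; Its Detector component hides the actor and disables Mesh collision on begin overlap, then restores both on end overlap.
; The check is an exact class match, and any matching end overlap restores the wall without counting remaining overlaps.
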(event `self.Detector.OnComponentBeginOverlap`
  (params (OverlappedComponent :type "PrimitiveComponent Object Reference") (OtherActor :type "Actor Object Reference") (OtherComp :type "PrimitiveComponent Object Reference") (OtherBodyIndex :type Integer) (bFromSweep :type Boolean) (SweepResult :type "HitResult Structure (by ref)"))
  (if (== (`GameplayStatics.GetObjectClass` OtherActor) "BP_Wall_Generic_C")
    (`self.SetActorHiddenInGame` true)
    (`PrimitiveComponent.SetCollisionEnabled` (`self.Mesh`) "NoCollision")))

(event `self.Detector.OnComponentEndOverlap`
  (params (OverlappedComponent :type "PrimitiveComponent Object Reference") (OtherActor :type "Actor Object Reference") (OtherComp :type "PrimitiveComponent Object Reference") (OtherBodyIndex :type Integer))
  (if (== (`GameplayStatics.GetObjectClass` OtherActor) "BP_Wall_Generic_C")
    (`self.SetActorHiddenInGame` false)
    (`PrimitiveComponent.SetCollisionEnabled` (`self.Mesh`) "QueryAndPhysics")))

(fn `UserConstructionScript`)