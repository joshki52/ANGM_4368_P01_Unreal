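; BP_Interactable_CRT is an interactable CRT monitor that the player can toggle on and off.
; Being targeted for interaction turns custom depth rendering on for the mesh and losing target turns it off.
; Primary interaction runs a FlipFlop that swaps the screen between on and off materials, playing a different sound at the actor's location for each state.
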(event `/Game/_Game/Blueprints/BPI_Interact.InteractTargetBegin`
  (`PrimitiveComponent.SetRenderCustomDepth` (`self.Interactable Mesh`) true))

(event `/Game/_Game/Blueprints/BPI_Interact.InteractTargetEnd`
  (`PrimitiveComponent.SetRenderCustomDepth` (`self.Interactable Mesh`) false))

(event `/Game/_Game/Blueprints/BPI_Interact.InteractPrimary`
  (bind _sm_crt_screen (`self.SM_CRT_Screen`))
  (`/Engine/EditorBlueprintResources/StandardMacros.FlipFlop`
    (:`A`
      (`PrimitiveComponent.SetMaterial` _sm_crt_screen 0 "/Game/_Game/Assets/Materials/MI_CRT_Screen_On.MI_CRT_Screen_On")
      (`GameplayStatics.PlaySoundAtLocation` "/Game/_Game/Assets/SFX/SFX_Terminal.SFX_Terminal" (`self.K2_GetActorLocation`) (struct) 1.0 1.0 0.0 null null null null))
    (:`B`
      (`PrimitiveComponent.SetMaterial` _sm_crt_screen 0 "/Game/_Game/Assets/Materials/MI_CRT_Screen_Off.MI_CRT_Screen_Off")
      (`GameplayStatics.PlaySoundAtLocation` "/Game/_Game/Assets/SFX/SFX_Deconstruct_Alternate.SFX_Deconstruct_Alternate" (`self.K2_GetActorLocation`) (struct) 1.0 1.0 0.0 null null null null))))

(fn `UserConstructionScript`
  (`parent.UserConstructionScript`))