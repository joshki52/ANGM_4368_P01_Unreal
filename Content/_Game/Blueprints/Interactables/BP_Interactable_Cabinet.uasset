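; Interactable cabinet that toggles open and closed on primary interaction, switching its point light on while open.
; Each interaction sends a signal, plays a sound and sets a target rotation for the mesh, pitched 90 degrees when open.
; Tick eases the mesh toward that target with RInterpTo, at a speed derived from ToggleDuration.
; Interaction targeting toggles custom depth rendering on the mesh.
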(event `/Game/_Game/Blueprints/BPI_Interact.InteractTargetBegin`
  (`PrimitiveComponent.SetRenderCustomDepth` (`self.Interactable Mesh`) true))

(event `/Game/_Game/Blueprints/BPI_Interact.InteractTargetEnd`
  (`PrimitiveComponent.SetRenderCustomDepth` (`self.Interactable Mesh`) false))

(event `/Game/_Game/Blueprints/BPI_Interact.InteractPrimary`
  (bind _pointlight (`self.PointLight`))
  (`self.Send Signal`)
  (if (`self.Open`)
    (set `self.Open` false)
    (set `self.Target Rotation` (`KismetMathLibrary.MakeRotator` 0.0))
    (`SceneComponent.SetVisibility` _pointlight false false)
    (else
      (set `self.Open` true)
      (set `self.Target Rotation` (`KismetMathLibrary.MakeRotator` 0.0 90.0))
      (`SceneComponent.SetVisibility` _pointlight true false)))
  (`GameplayStatics.PlaySoundAtLocation` "/Game/_Game/Assets/SFX/SFX_Deconstruct_Alternate.SFX_Deconstruct_Alternate" (`self.K2_GetActorLocation`) (struct) 1.0 1.0 0.0 null null null null))

(event `self.ReceiveTick`
  (params (DeltaSeconds :type "Float (single-precision)"))
  (bind _interactable_mesh (`self.Interactable Mesh`))
  (if (!= (`SceneComponent.RelativeRotation` (`self.Interactable Mesh`)) (`self.Target Rotation`) :`ErrorTolerance` 1.0)
    (`SceneComponent.K2_SetRelativeRotation` _interactable_mesh (`KismetMathLibrary.RInterpTo` (`SceneComponent.RelativeRotation` _interactable_mesh) (`self.Target Rotation`) DeltaSeconds (/ 1.0 (`self.Toggle Duration`))) false false)))

(fn `UserConstructionScript`
  (`parent.UserConstructionScript`))