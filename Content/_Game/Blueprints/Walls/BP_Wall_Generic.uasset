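; BP_Wall_Generic is a wall actor that hides itself while its Detector overlaps another actor of the same class or a subclass.
; Detector begin overlap hides Mesh and disables its collision; end overlap shows it again with query and physics collision.
; Each end overlap restores Mesh directly, with no count of remaining overlaps.
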(event `self.Detector.OnComponentBeginOverlap`
  (params (OverlappedComponent :type "PrimitiveComponent Object Reference") (OtherActor :type "Actor Object Reference") (OtherComp :type "PrimitiveComponent Object Reference") (OtherBodyIndex :type Integer) (bFromSweep :type Boolean) (SweepResult :type "HitResult Structure (by ref)"))
  (bind _mesh (`self.Mesh`))
  (if (`KismetMathLibrary.ClassIsChildOf` (`GameplayStatics.GetObjectClass` OtherActor) "BP_Wall_Generic_C")
    (`SceneComponent.SetHiddenInGame` _mesh true false)
    (`PrimitiveComponent.SetCollisionEnabled` _mesh "NoCollision")))

(event `self.Detector.OnComponentEndOverlap`
  (params (OverlappedComponent :type "PrimitiveComponent Object Reference") (OtherActor :type "Actor Object Reference") (OtherComp :type "PrimitiveComponent Object Reference") (OtherBodyIndex :type Integer))
  (bind _mesh (`self.Mesh`))
  (if (`KismetMathLibrary.ClassIsChildOf` (`GameplayStatics.GetObjectClass` OtherActor) "BP_Wall_Generic_C")
    (`SceneComponent.SetHiddenInGame` _mesh false false)
    (`PrimitiveComponent.SetCollisionEnabled` _mesh "QueryAndPhysics")))

(fn `UserConstructionScript`)