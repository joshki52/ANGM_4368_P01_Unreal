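; Parent Blueprint for modular rooms that flags overlaps and opens walls where another room adjoins.
; A room detector sets IsClipping when overlapping any other actor, while four wall detectors hide their wall mesh and disable its collision through EnableComponent.
; Only the north wall restores on end overlap; the other three restore branches are unwired.
; The room check compares exact class, so child classes fail it.
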(event `self.Room Detector.OnComponentBeginOverlap`
  (params (OverlappedComponent :type "PrimitiveComponent Object Reference") (OtherActor :type "Actor Object Reference") (OtherComp :type "PrimitiveComponent Object Reference") (OtherBodyIndex :type Integer) (bFromSweep :type Boolean) (SweepResult :type "HitResult Structure (by ref)"))
  (`self.Test If Self` OtherActor self
    (:`False`
      (set `self.Is Clipping` true)
      (`KismetSystemLibrary.PrintString` "Is Clipping"))))

(event `self.Room Detector.OnComponentEndOverlap`
  (params (OverlappedComponent :type "PrimitiveComponent Object Reference") (OtherActor :type "Actor Object Reference") (OtherComp :type "PrimitiveComponent Object Reference") (OtherBodyIndex :type Integer))
  (`self.Test If Self` OtherActor self
    (:`False`
      (set `self.Is Clipping` false)
      (`KismetSystemLibrary.PrintString` "Is Not Clipping"))))

(event `self.Wall N Detector.OnComponentBeginOverlap`
  (params (OverlappedComponent :type "PrimitiveComponent Object Reference") (OtherActor :type "Actor Object Reference") (OtherComp :type "PrimitiveComponent Object Reference") (OtherBodyIndex :type Integer) (bFromSweep :type Boolean) (SweepResult :type "HitResult Structure (by ref)"))
  (`self.Test Actor Type` OtherActor "BP_Room_ParentClass_C"
    (:`True`
      (`self.Enable Component` (`self.Wall N Mesh`)))))

(event `self.Wall N Detector.OnComponentEndOverlap`
  (params (OverlappedComponent :type "PrimitiveComponent Object Reference") (OtherActor :type "Actor Object Reference") (OtherComp :type "PrimitiveComponent Object Reference") (OtherBodyIndex :type Integer))
  (`self.Test Actor Type` OtherActor "BP_Room_ParentClass_C"
    (:`True`
      (`self.Enable Component` (`self.Wall N Mesh`) true))))

(event `self.Wall S Detector.OnComponentBeginOverlap`
  (params (OverlappedComponent :type "PrimitiveComponent Object Reference") (OtherActor :type "Actor Object Reference") (OtherComp :type "PrimitiveComponent Object Reference") (OtherBodyIndex :type Integer) (bFromSweep :type Boolean) (SweepResult :type "HitResult Structure (by ref)"))
  (`self.Test Actor Type` OtherActor "BP_Room_ParentClass_C"
    (:`True`
      (`self.Enable Component` (`self.Wall S Mesh`)))))

(event `self.Wall S Detector.OnComponentEndOverlap`
  (params (OverlappedComponent :type "PrimitiveComponent Object Reference") (OtherActor :type "Actor Object Reference") (OtherComp :type "PrimitiveComponent Object Reference") (OtherBodyIndex :type Integer)))

(event `self.Wall E Detector.OnComponentBeginOverlap`
  (params (OverlappedComponent :type "PrimitiveComponent Object Reference") (OtherActor :type "Actor Object Reference") (OtherComp :type "PrimitiveComponent Object Reference") (OtherBodyIndex :type Integer) (bFromSweep :type Boolean) (SweepResult :type "HitResult Structure (by ref)"))
  (`self.Test Actor Type` OtherActor "BP_Room_ParentClass_C"
    (:`True`
      (`self.Enable Component` (`self.Wall E Mesh`)))))

(event `self.Wall E Detector.OnComponentEndOverlap`
  (params (OverlappedComponent :type "PrimitiveComponent Object Reference") (OtherActor :type "Actor Object Reference") (OtherComp :type "PrimitiveComponent Object Reference") (OtherBodyIndex :type Integer)))

(event `self.Wall W Detector.OnComponentBeginOverlap`
  (params (OverlappedComponent :type "PrimitiveComponent Object Reference") (OtherActor :type "Actor Object Reference") (OtherComp :type "PrimitiveComponent Object Reference") (OtherBodyIndex :type Integer) (bFromSweep :type Boolean) (SweepResult :type "HitResult Structure (by ref)"))
  (`self.Test Actor Type` OtherActor "BP_Room_ParentClass_C"
    (:`True`
      (`self.Enable Component` (`self.Wall W Mesh`)))))

(event `self.Wall W Detector.OnComponentEndOverlap`
  (params (OverlappedComponent :type "PrimitiveComponent Object Reference") (OtherActor :type "Actor Object Reference") (OtherComp :type "PrimitiveComponent Object Reference") (OtherBodyIndex :type Integer)))

(fn `Enable Component`
  (params (`Target Component` :type "PrimitiveComponent Object Reference") (`New Enabled` :type Boolean))
  (if `New Enabled`
    (`PrimitiveComponent.SetCollisionEnabled` `Target Component` "QueryAndPhysics")
    (else
      (`PrimitiveComponent.SetCollisionEnabled` `Target Component` "NoCollision")))
  (`SceneComponent.SetHiddenInGame` `Target Component` (not `New Enabled`) false))

(fn `UserConstructionScript`)