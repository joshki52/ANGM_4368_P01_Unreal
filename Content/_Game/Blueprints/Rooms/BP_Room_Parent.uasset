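; BP_Room_Parent is a room Blueprint, named as a parent class, that records its static meshes and can switch components on or off.
; The construction script adds the root's direct children whose class is exactly StaticMeshComponent to the StaticMeshes array.
; EnableComponent toggles a given component's collision and in-game visibility together, without propagating visibility to children.
; Nothing in these graphs calls EnableComponent or reads the array.
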(fn `Enable Component`
  (params (`Target Component` :type "PrimitiveComponent Object Reference") (`New Enabled` :type Boolean))
  (if `New Enabled`
    (`PrimitiveComponent.SetCollisionEnabled` `Target Component` "QueryAndPhysics")
    (else
      (`PrimitiveComponent.SetCollisionEnabled` `Target Component` "NoCollision")))
  (`SceneComponent.SetHiddenInGame` `Target Component` (not `New Enabled`) false))

(fn `UserConstructionScript`
  (for _array_element (`SceneComponent.GetChildrenComponents` (`self.DefaultSceneRoot`) false)
    (if (== (`GameplayStatics.GetObjectClass` _array_element) "/Script/Engine.StaticMeshComponent")
      (bind _asstatic_mesh_component (cast `StaticMeshComponent` _array_element)
        (:`then`
          (`KismetArrayLibrary.Array_Add` (`self.Static Meshes`) _asstatic_mesh_component))
        (:`CastFailed`
          (`KismetSystemLibrary.PrintString` "Could not record static mesh to array!"))))))